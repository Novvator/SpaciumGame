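; Paper2D door Blueprint that opens when a 2DSideScrollerCharacter carrying a key enters its trigger box.
; Box1's overlap checks the character's HasKey flag and the door's IsOpen state, then consumes the key and plays the door flipbook.
; After a short delay it switches to the open flipbook, sets the blocking Box to overlap all channels and marks itself open.
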(event OnComponentBeginOverlap(Box1)
  (params (OverlappedComponent :type Primitive%20Component%20Object%20Reference) (OtherActor :type Actor%20Object%20Reference) (OtherComp :type Primitive%20Component%20Object%20Reference) (OtherBodyIndex :type Integer) (bFromSweep :type Boolean) (SweepResult :type Hit%20Result%20Structure%20%28by%20ref%29))
  (bind _as2dside_scroller_character (Utilities|Casting|CastTo2DSideScrollerCharacter OtherActor))
  (if (Variables|/Game/2DSideScrollerBP/character/2DSideScrollerCharacter.2DSideScrollerCharacter_C|GethasKey _as2dside_scroller_character)
    (if (not (Variables|Default|GetisOpen))
      (Sprite|SetFlipbook (Variables|Default|GetPaperFlipbook) "/Game/items/door/flipbooks/door_flipbook.door_flipbook")
      (Variables|/Game/2DSideScrollerBP/character/2DSideScrollerCharacter.2DSideScrollerCharacter_C|SethasKey _as2dside_scroller_character false)
      (Utilities|FlowControl|Delay 0.6666)
      (Sprite|SetFlipbook (Variables|Default|GetPaperFlipbook) "/Game/items/door/flipbooks/door_open_flipbook.door_open_flipbook")
      (Collision|SetCollisionResponsetoAllChannels (Variables|Default|GetBox) "ECR_Overlap")
      (Variables|Default|SetisOpen true))))

(event EventBeginPlay)

(event Collision|EventActorBeginOverlap
  (params (OtherActor :type Actor%20Object%20Reference)))

(event EventTick
  (params (DeltaSeconds :type Float%20%28single-precision%29)))

(fn ConstructionScript)